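; BP_Area is a test area actor that applies the GE_HealthDrain gameplay effect to the player while its Box is overlapped.
; On BeginPlay it binds the Box overlap events; begin overlap applies the effect through the player's Ability System Component and stores the handle in NewVar.
; End overlap removes all stacks using that handle.
; Both events target player pawn 0 regardless of which actor overlaps.
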(event Custom|OnComponentBeginOverlap_이벤트
  (params (OverlappedComponent :type Primitive%20Component%20Object%20Reference) (OtherActor :type Actor%20Object%20Reference) (OtherComp :type Primitive%20Component%20Object%20Reference) (OtherBodyIndex :type Integer) (bFromSweep :type Boolean) (SweepResult :type Hit%20Result%20Structure%20%28by%20ref%29))
  (bind _returnvalue (GameplayEffects|ApplyGameplayEffectToSelf :self (Ability|GetAbilitySystemComponent (Game|Player|GetPlayerPawn 0)) :GameplayEffectClass "/Game/Blueprints/GAS/Effect/GE_HealthDrain.GE_HealthDrain_C"))
  (Variables|Default|SetNewVar _returnvalue))

(event Custom|OnComponentEndOverlap_이벤트
  (params (OverlappedComponent :type Primitive%20Component%20Object%20Reference) (OtherActor :type Actor%20Object%20Reference) (OtherComp :type Primitive%20Component%20Object%20Reference) (OtherBodyIndex :type Integer))
  (GameplayEffects|RemoveActiveGameplayEffect (Ability|GetAbilitySystemComponent (Game|Player|GetPlayerPawn 0)) (Variables|Default|GetNewVar) -1))

(event EventBeginPlay
  (bind _box (Variables|Default|GetBox))
  (Collision|AssignOnComponentBeginOverlap _box (delegate Custom|OnComponentBeginOverlap_이벤트))
  (Collision|AssignOnComponentEndOverlap _box (delegate Custom|OnComponentEndOverlap_이벤트)))

(fn ConstructionScript)