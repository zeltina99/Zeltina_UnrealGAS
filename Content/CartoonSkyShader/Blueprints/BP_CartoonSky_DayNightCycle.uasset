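; Cartoon sky actor that picks a cloud-type material and colors sun, moon, sky light and height fog to match.
; Colors are sampled from per-type curves using the sun direction's dot product with up.
; BeginPlay sets night if a SkyAtmosphere exists; events drive timelines for sunrise and moon fade-out.
; The continuous DayNightCycle function is disconnected, as Tick and the editor update branch are empty.
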(event Custom|FadeOutMoon
  (params (Times :type Float%20%28double-precision%29))
  (bind _returnvalue (Rendering|Material|CreateDynamicMaterialInstance (Variables|Default|GetCartoonSky) 0 (Rendering|Material|GetMaterial (Variables|Default|GetCartoonSky) 0) "None" :!class /Script/Engine.PrimitiveComponent))
  (Variables|Default|SetMID_MoonIntensity _returnvalue)
  (bind _newtrack_0 (Timeline|FadeOutMoonIntencity Play)
    (:Update
      (Rendering|Material|SetScalarParameterValue (Variables|Default|GetMID_MoonIntensity) "Moon Intensity at Night" _newtrack_0 :!class /Script/Engine.MaterialInstanceDynamic))))

(event Custom|StartSunRising
  (params (SunTimers :type Float%20%28double-precision%29))
  (CallFunction|RiseSun)
  (bind _newtrack_0 (Timeline|SunRiseTimeline Play)
    (:Update
      (Transformation|SetActorRotation (Variables|Sun|GetSunLight) (Math|Rotator|MakeRotator 0.0 _newtrack_0 0.0)))))

(event EventBeginPlay
  (bind _returnvalue (Actor|GetActorOfClass "/Script/Engine.SkyAtmosphere"))
  (Utilities|IsValid _returnvalue
    (:Is%20Valid
      (CallFunction|NightSetting)
      (Transformation|SetActorRotation (Variables|Sun|GetSunLight) "90.000000,0.000000,0.000000"))
    (:Is%20Not%20Valid
      (Development|PrintString "Place Sky Atmosphere actor in the scene" true true "(R=1.000000,G=0.000000,B=0.000000,A=1.000000)" 3e+01))))

(event EventTick
  (params (DeltaSeconds :type Float%20%28single-precision%29)))

(fn ConstructionScript
  (Rendering|Material|SetMaterial (Variables|Default|GetCartoonSky) 0 (Utilities|Select :Index (Variables|DayNightCycle|GetCloudTypes) :NewEnumerator0 "/Game/Assets/SkyAtmosphere/CartoonSkyShader/Materials/CartoonSkyInstances/MI_CartoonSky_Type_1_High_Detail.MI_CartoonSky_Type_1_High_Detail" :NewEnumerator1 "/Game/Assets/SkyAtmosphere/CartoonSkyShader/Materials/CartoonSkyInstances/MI_CartoonSky_Type_1_Low_Detail.MI_CartoonSky_Type_1_Low_Detail" :NewEnumerator15 0 :NewEnumerator2 "/Game/Assets/SkyAtmosphere/CartoonSkyShader/Materials/CartoonSkyInstances/MI_CartoonSky_Type_2_High_Detail.MI_CartoonSky_Type_2_High_Detail" :NewEnumerator3 "/Game/Assets/SkyAtmosphere/CartoonSkyShader/Materials/CartoonSkyInstances/MI_CartoonSky_Type_2_Low_Detail.MI_CartoonSky_Type_2_Low_Detail" :NewEnumerator4 0 :NewEnumerator5 "/Game/Assets/SkyAtmosphere/CartoonSkyShader/Materials/CartoonSkyInstances/MI_CartoonSky_Type_3_High_Detail.MI_CartoonSky_Type_3_High_Detail" :NewEnumerator6 "/Game/Assets/SkyAtmosphere/CartoonSkyShader/Materials/CartoonSkyInstances/MI_CartoonSky_Type_3_Low_Detail.MI_CartoonSky_Type_3_Low_Detail" :NewEnumerator16 0 :NewEnumerator7 "/Game/Assets/SkyAtmosphere/CartoonSkyShader/Materials/CartoonSkyInstances/MI_CartoonSky_Type_4_High_Detail.MI_CartoonSky_Type_4_High_Detail" :NewEnumerator8 "/Game/Assets/SkyAtmosphere/CartoonSkyShader/Materials/CartoonSkyInstances/MI_CartoonSky_Type_4_Low_Detail.MI_CartoonSky_Type_4_Low_Detail" :NewEnumerator10 0 :NewEnumerator11 "/Game/Assets/SkyAtmosphere/CartoonSkyShader/Materials/CartoonSkyInstances/MI_CartoonSky_Type_5_High_Detail.MI_CartoonSky_Type_5_High_Detail" :NewEnumerator12 "/Game/Assets/SkyAtmosphere/CartoonSkyShader/Materials/CartoonSkyInstances/MI_CartoonSky_Type_5_Low_Detail.MI_CartoonSky_Type_5_Low_Detail"))
  (if (Variables|DayNightCycle|GetUpdate%20Sky%20in%20the%20editor)
    _
    (else
      _))
  (Variables|DayNightCycle|SetUpdate%20Sky%20in%20the%20editor false))

(fn DayNightCycle
  (params (Delta :type Float%20%28double-precision%29))
  (bind _defaultsceneroot (Variables|Default|GetDefaultSceneRoot))
  (bind _moonlight (Variables|Moon|GetMoonLight))
  (bind _skylight (Variables|Skylight|GetSkylight))
  (bind _height_fog (Variables|HeightFog|GetHeight%20Fog))
  (bind _sunlight (Variables|Sun|GetSunLight))
  (bind _returnvalue (Math|Vector|GetUpVector _defaultsceneroot))
  (bind _lightcomponent (Variables|/Script/Engine.Light|GetLightComponent _sunlight))
  (bind _lightcomponent_2 (Variables|/Script/Engine.Light|GetLightComponent _moonlight))
  (bind _lightcomponent_3 (Variables|/Script/Engine.Light|GetLightComponent _sunlight))
  (bind _returnvalue_2 (Math|Vector|GetForwardVector _lightcomponent))
  (bind _returnvalue_3 (* _returnvalue_2 -1.0))
  (bind _returnvalue_4 (Math|Vector|DotProduct _returnvalue_3 _returnvalue))
  (bind _returnvalue_5 (+ _returnvalue_4 0.5))
  (bind _returnvalue_6 (Math|Float|NormalizetoRange _returnvalue_5 0.0 1.0))
  (Utilities|FlowControl|Sequence
    (:then_0
      (switch Utilities|FlowControl|Switch|SwitchonE_CloudTypes (Variables|DayNightCycle|GetCloudTypes)
        (:NewEnumerator0
          (Variables|Sun|SetSun%20Light%20Color (Variables|Sun|GetSun%20Light%20Color%20Type%201) :!label _label)
          (Variables|Moon|SetMoon%20Light%20Color (Variables|Moon|GetMoon%20Light%20Color%20Type%201))
          (Variables|Skylight|SetSkylight%20Color (Variables|Skylight|GetSkylight%20Color%20Type%201))
          (Variables|HeightFog|SetHeight%20Fog%20Color (Variables|HeightFog|GetHeight%20Fog%20Type%201)))
        (:NewEnumerator1
          (goto _label))
        (:NewEnumerator2
          (Variables|Sun|SetSun%20Light%20Color (Variables|Sun|GetSun%20Light%20Color%20Type%202) :!label _label_2)
          (Variables|Moon|SetMoon%20Light%20Color (Variables|Moon|GetMoon%20Light%20Color%20Type%202))
          (Variables|Skylight|SetSkylight%20Color (Variables|Skylight|GetSkylight%20Color%20Type%202))
          (Variables|HeightFog|SetHeight%20Fog%20Color (Variables|HeightFog|GetHeight%20Fog%20Type%202)))
        (:NewEnumerator3
          (goto _label_2))
        (:NewEnumerator5
          (Variables|Sun|SetSun%20Light%20Color (Variables|Sun|GetSun%20Light%20Color%20Type%203) :!label _label_3)
          (Variables|Moon|SetMoon%20Light%20Color (Variables|Moon|GetMoon%20Light%20Color%20Type%203))
          (Variables|Skylight|SetSkylight%20Color (Variables|Skylight|GetSkylight%20Color%20Type%203))
          (Variables|HeightFog|SetHeight%20Fog%20Color (Variables|HeightFog|GetHeight%20Fog%20Type%203)))
        (:NewEnumerator6
          (goto _label_3))
        (:NewEnumerator7
          (Variables|Sun|SetSun%20Light%20Color (Variables|Sun|GetSun%20Light%20Color%20Type%204) :!label _label_4)
          (Variables|Moon|SetMoon%20Light%20Color (Variables|Moon|GetMoon%20Light%20Color%20Type%204))
          (Variables|Skylight|SetSkylight%20Color (Variables|Skylight|GetSkylight%20Color%20Type%204))
          (Variables|HeightFog|SetHeight%20Fog%20Color (Variables|HeightFog|GetHeight%20Fog%20Type%204)))
        (:NewEnumerator8
          (goto _label_4))
        (:NewEnumerator11
          (Variables|Sun|SetSun%20Light%20Color (Variables|Sun|GetSun%20Light%20Color%20Type%205) :!label _label_5)
          (Variables|Moon|SetMoon%20Light%20Color (Variables|Moon|GetMoon%20Light%20Color%20Type%205))
          (Variables|Skylight|SetSkylight%20Color (Variables|Skylight|GetSkylight%20Color%20Type%205))
          (Variables|HeightFog|SetHeight%20Fog%20Color (Variables|HeightFog|GetHeight%20Fog%20Type%205)))
        (:NewEnumerator12
          (goto _label_5))))
    (:then_1
      (Utilities|IsValid _sunlight
        (:Is%20Valid
          (Transformation|AddLocalRotation _lightcomponent_3 (Math|Rotator|MakeRotator 0.0 (Variables|Default|GetSpeed) 0.0) false false)
          (Rendering|Components|Light|SetLightColor _lightcomponent_3 (Math|Curves|GetLinearColorValue (Variables|Sun|GetSun%20Light%20Color) _returnvalue_6) true)
          (Utilities|IsValid _skylight
            (:Is%20Valid
              (Rendering|Components|Light|SetLightColor (Variables|/Script/Engine.SkyLight|GetLightComponent _skylight) (Math|Curves|GetLinearColorValue (Variables|Skylight|GetSkylight%20Color) _returnvalue_6))
              (Utilities|IsValid _height_fog
                (:Is%20Valid
                  (Class|ExponentialHeightFogComponent|SetFogInscatteringColor (Variables|/Script/Engine.ExponentialHeightFog|GetComponent _height_fog) (Math|Curves|GetLinearColorValue (Variables|HeightFog|GetHeight%20Fog%20Color) _returnvalue_6)))
                (:Is%20Not%20Valid
                  (Development|PrintString "Set a Height Fog in BP_CartoonSky_DayNightCycle" true true "(R=0.000000,G=0.660000,B=1.000000,A=1.000000)" 0.001))))
            (:Is%20Not%20Valid
              (Development|PrintString "Set a Sky Light in BP_CartoonSky_DayNightCycle" true true "(R=0.000000,G=0.660000,B=1.000000,A=1.000000)" 0.001))))
        (:Is%20Not%20Valid
          (Development|PrintString "Set a Sun Light in BP_CartoonSky_DayNightCycle" true true "(R=0.000000,G=0.660000,B=1.000000,A=1.000000)" 0.001))))
    (:then_2
      (Utilities|IsValid _moonlight
        (:Is%20Valid
          (Rendering|Components|Light|SetLightColor _lightcomponent_2 (Math|Curves|GetLinearColorValue (Variables|Moon|GetMoon%20Light%20Color) _returnvalue_6) true)
          (if (Variables|DayNightCycle|GetMoon%20Rotation?)
            (Transformation|AddWorldRotation _lightcomponent_2 (Math|Rotator|MakeRotator 0.0 0.0 (Variables|Default|GetSpeed)) false false)))
        (:Is%20Not%20Valid
          (Development|PrintString "Set a Moon Light in BP_CartoonSky_DayNightCycle" true true "(R=0.000000,G=0.660000,B=1.000000,A=1.000000)" 0.001))))))

(fn NightSetting
  (bind _defaultsceneroot (Variables|Default|GetDefaultSceneRoot))
  (bind _moonlight (Variables|Moon|GetMoonLight))
  (bind _skylight (Variables|Skylight|GetSkylight))
  (bind _height_fog (Variables|HeightFog|GetHeight%20Fog))
  (bind _sunlight (Variables|Sun|GetSunLight))
  (bind _returnvalue (Math|Vector|GetUpVector _defaultsceneroot))
  (bind _lightcomponent (Variables|/Script/Engine.Light|GetLightComponent _sunlight))
  (bind _lightcomponent_2 (Variables|/Script/Engine.Light|GetLightComponent _moonlight))
  (bind _returnvalue_2 (Math|Vector|GetForwardVector _lightcomponent))
  (bind _returnvalue_3 (* _returnvalue_2 -1.0))
  (bind _returnvalue_4 (Math|Vector|DotProduct _returnvalue_3 _returnvalue))
  (bind _returnvalue_5 (+ _returnvalue_4 0.5))
  (bind _returnvalue_6 (Math|Float|NormalizetoRange _returnvalue_5 0.0 1.0))
  (Utilities|FlowControl|Sequence
    (:then_0
      (switch Utilities|FlowControl|Switch|SwitchonE_CloudTypes (Variables|DayNightCycle|GetCloudTypes)
        (:NewEnumerator0
          (Variables|Sun|SetSun%20Light%20Color (Variables|Sun|GetSun%20Light%20Color%20Type%201) :!label _label)
          (Variables|Moon|SetMoon%20Light%20Color (Variables|Moon|GetMoon%20Light%20Color%20Type%201))
          (Variables|Skylight|SetSkylight%20Color (Variables|Skylight|GetSkylight%20Color%20Type%201))
          (Variables|HeightFog|SetHeight%20Fog%20Color (Variables|HeightFog|GetHeight%20Fog%20Type%201)))
        (:NewEnumerator1
          (goto _label))
        (:NewEnumerator2
          (Variables|Sun|SetSun%20Light%20Color (Variables|Sun|GetSun%20Light%20Color%20Type%202) :!label _label_2)
          (Variables|Moon|SetMoon%20Light%20Color (Variables|Moon|GetMoon%20Light%20Color%20Type%202))
          (Variables|Skylight|SetSkylight%20Color (Variables|Skylight|GetSkylight%20Color%20Type%202))
          (Variables|HeightFog|SetHeight%20Fog%20Color (Variables|HeightFog|GetHeight%20Fog%20Type%202)))
        (:NewEnumerator3
          (goto _label_2))
        (:NewEnumerator5
          (Variables|Sun|SetSun%20Light%20Color (Variables|Sun|GetSun%20Light%20Color%20Type%203) :!label _label_3)
          (Variables|Moon|SetMoon%20Light%20Color (Variables|Moon|GetMoon%20Light%20Color%20Type%203))
          (Variables|Skylight|SetSkylight%20Color (Variables|Skylight|GetSkylight%20Color%20Type%203))
          (Variables|HeightFog|SetHeight%20Fog%20Color (Variables|HeightFog|GetHeight%20Fog%20Type%203)))
        (:NewEnumerator6
          (goto _label_3))
        (:NewEnumerator7
          (Variables|Sun|SetSun%20Light%20Color (Variables|Sun|GetSun%20Light%20Color%20Type%204) :!label _label_4)
          (Variables|Moon|SetMoon%20Light%20Color (Variables|Moon|GetMoon%20Light%20Color%20Type%204))
          (Variables|Skylight|SetSkylight%20Color (Variables|Skylight|GetSkylight%20Color%20Type%204))
          (Variables|HeightFog|SetHeight%20Fog%20Color (Variables|HeightFog|GetHeight%20Fog%20Type%204)))
        (:NewEnumerator8
          (goto _label_4))
        (:NewEnumerator11
          (Variables|Sun|SetSun%20Light%20Color (Variables|Sun|GetSun%20Light%20Color%20Type%205) :!label _label_5)
          (Variables|Moon|SetMoon%20Light%20Color (Variables|Moon|GetMoon%20Light%20Color%20Type%205))
          (Variables|Skylight|SetSkylight%20Color (Variables|Skylight|GetSkylight%20Color%20Type%205))
          (Variables|HeightFog|SetHeight%20Fog%20Color (Variables|HeightFog|GetHeight%20Fog%20Type%205)))
        (:NewEnumerator12
          (goto _label_5))))
    (:then_1
      (Utilities|IsValid _sunlight
        (:Is%20Valid
          (Rendering|Components|Light|SetLightColor (Variables|/Script/Engine.Light|GetLightComponent _sunlight) (Math|Curves|GetLinearColorValue (Variables|Sun|GetSun%20Light%20Color) _returnvalue_6) true)
          (Utilities|IsValid _skylight
            (:Is%20Valid
              (Rendering|Components|Light|SetLightColor (Variables|/Script/Engine.SkyLight|GetLightComponent _skylight) (Math|Curves|GetLinearColorValue (Variables|Skylight|GetSkylight%20Color) _returnvalue_6))
              (Utilities|IsValid _height_fog
                (:Is%20Valid
                  (Class|ExponentialHeightFogComponent|SetFogInscatteringColor (Variables|/Script/Engine.ExponentialHeightFog|GetComponent _height_fog) (Math|Curves|GetLinearColorValue (Variables|HeightFog|GetHeight%20Fog%20Color) _returnvalue_6)))
                (:Is%20Not%20Valid
                  (Development|PrintString "Set a Height Fog in BP_CartoonSky_DayNightCycle" true true "(R=0.000000,G=0.660000,B=1.000000,A=1.000000)" 0.001))))
            (:Is%20Not%20Valid
              (Development|PrintString "Set a Sky Light in BP_CartoonSky_DayNightCycle" true true "(R=0.000000,G=0.660000,B=1.000000,A=1.000000)" 0.001))))
        (:Is%20Not%20Valid
          (Development|PrintString "Set a Sun Light in BP_CartoonSky_DayNightCycle" true true "(R=0.000000,G=0.660000,B=1.000000,A=1.000000)" 0.001))))
    (:then_2
      (Utilities|IsValid _moonlight
        (:Is%20Valid
          (Rendering|Components|Light|SetLightColor _lightcomponent_2 (Math|Curves|GetLinearColorValue (Variables|Moon|GetMoon%20Light%20Color) _returnvalue_6) true)
          (if (Variables|DayNightCycle|GetMoon%20Rotation?)
            (Transformation|AddWorldRotation _lightcomponent_2 (Math|Rotator|MakeRotator 0.0 0.0 (Variables|Default|GetSpeed)) false false)))
        (:Is%20Not%20Valid
          (Development|PrintString "Set a Moon Light in BP_CartoonSky_DayNightCycle" true true "(R=0.000000,G=0.660000,B=1.000000,A=1.000000)" 0.001))))))

(fn RiseSun
  (bind _defaultsceneroot (Variables|Default|GetDefaultSceneRoot))
  (bind _moonlight (Variables|Moon|GetMoonLight))
  (bind _skylight (Variables|Skylight|GetSkylight))
  (bind _height_fog (Variables|HeightFog|GetHeight%20Fog))
  (bind _sunlight (Variables|Sun|GetSunLight))
  (bind _returnvalue (Math|Vector|GetUpVector _defaultsceneroot))
  (bind _lightcomponent (Variables|/Script/Engine.Light|GetLightComponent _sunlight))
  (bind _returnvalue_2 (Math|Vector|GetForwardVector _lightcomponent))
  (bind _returnvalue_3 (* _returnvalue_2 -1.0))
  (bind _returnvalue_4 (Math|Vector|DotProduct _returnvalue_3 _returnvalue))
  (bind _returnvalue_5 (+ _returnvalue_4 0.5))
  (bind _returnvalue_6 (Math|Float|NormalizetoRange _returnvalue_5 0.0 1.0))
  (Utilities|FlowControl|Sequence
    (:then_0
      (Utilities|IsValid _sunlight
        (:Is%20Valid
          (Transformation|SetActorRotation _sunlight "10.000000,0.000000,0.000000")
          (Rendering|Components|Light|SetLightColor (Variables|/Script/Engine.Light|GetLightComponent _sunlight) (Math|Curves|GetLinearColorValue (Variables|Sun|GetSun%20Light%20Color) _returnvalue_6) true)
          (Utilities|IsValid _skylight
            (:Is%20Valid
              (Rendering|Components|Light|SetLightColor (Variables|/Script/Engine.SkyLight|GetLightComponent _skylight) (Math|Curves|GetLinearColorValue (Variables|Skylight|GetSkylight%20Color) _returnvalue_6))
              (Utilities|IsValid _height_fog
                (:Is%20Valid
                  (Class|ExponentialHeightFogComponent|SetFogInscatteringColor (Variables|/Script/Engine.ExponentialHeightFog|GetComponent _height_fog) (Math|Curves|GetLinearColorValue (Variables|HeightFog|GetHeight%20Fog%20Color) _returnvalue_6)))
                (:Is%20Not%20Valid
                  (Development|PrintString "Set a Height Fog in BP_CartoonSky_DayNightCycle" true true "(R=0.000000,G=0.660000,B=1.000000,A=1.000000)" 0.001))))
            (:Is%20Not%20Valid
              (Development|PrintString "Set a Sky Light in BP_CartoonSky_DayNightCycle" true true "(R=0.000000,G=0.660000,B=1.000000,A=1.000000)" 0.001))))
        (:Is%20Not%20Valid
          (Development|PrintString "Set a Sun Light in BP_CartoonSky_DayNightCycle" true true "(R=0.000000,G=0.660000,B=1.000000,A=1.000000)" 0.001))))
    (:then_1
      (Utilities|IsValid _moonlight
        (:Is%20Valid
          (Rendering|Components|Light|SetLightColor (Variables|/Script/Engine.Light|GetLightComponent _moonlight) (Math|Curves|GetLinearColorValue (Variables|Moon|GetMoon%20Light%20Color) _returnvalue_6) true))))))